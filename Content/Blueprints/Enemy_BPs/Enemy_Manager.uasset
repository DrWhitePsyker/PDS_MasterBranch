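; Enemy manager that spreads enemy player-sight checks across frames to limit per-tick cost.
; FeedToUpdateArray deals enemies round-robin into a fixed set of buckets, stored as an array of array structs.
; Each Tick processes one bucket, calling UpdatePlayerSight on Enemy_Core members not in combat, then advances to the next, wrapping around.
; Failed casts print a warning, and a note flags that Enemy_Core children need patching.
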(event Custom|FeedToUpdateArray
  (Utilities|Array|Add (Utilities|Struct|BreakActorArrayStruct (Utilities|Array|Get(acopy) (Variables|Default|GetEnemyUpdateArrayY) (Variables|Default|GetSorting%20Pass))) (Variables|Default|GetEnemyNeedingSorting))
  (bind _result (Math|Integer|IncrementInt (Variables|Default|GetSorting%20Pass))
    (:%20%20
      (if (> _result 18)
        (Variables|Default|SetSorting%20Pass 0)))))

(event EventTick
  (params (DeltaSeconds :type Float%20%28single-precision%29))
  ;[1 1 1] THIS NEEDS PATCHING FOR ENEMY CORE CHILDREN
  (for _array_element (Utilities|Struct|BreakActorArrayStruct (Utilities|Array|Get(acopy) (Variables|Default|GetEnemyUpdateArrayY) (Variables|Default|GetTickPass)))
    (bind _asenemy_core (Utilities|Casting|CastToEnemy_Core _array_element)
      (:then
        (if (not (Variables|/Game/Blueprints/Enemy_BPs/Enemy_Core.Enemy_Core_C|GetInCombat? _asenemy_core))
          (Default|UpdatePlayerSight _asenemy_core)))
      (:CastFailed
        (Development|PrintString "EnemyManager: Pass object is not enemy_core?"))))
  (bind _result (Math|Integer|IncrementInt (Variables|Default|GetTickPass))
    (:%20%20
      (if (> _result 18)
        (Variables|Default|SetTickPass 0)))))

(fn ConstructionScript)