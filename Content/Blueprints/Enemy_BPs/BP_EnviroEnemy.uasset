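; BP_EnviroEnemy is an enemy Blueprint that periodically spawns pools under its feet as it exists in the level.
; Tick runs the parent logic, then a half-second Delay throttles calls to the SpawnPool event to roughly twice per second.
; SpawnPool spawns an actor at the PoolSpawner component's world transform; BeginPlay and the construction script only call their parents.
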(event Custom|SpawnPool
  ;[1 1 1] Added 11/03/2020 - spawn pools underfeet
  (Game|SpawnActorfromClass "/Game/Blueprints/Enemy_BPs/BP_DamagingPool.BP_DamagingPool_C" (Transformation|GetWorldTransform (Variables|Default|GetPoolSpawner)) "Undefined" 0 0))

(event EventBeginPlay
  (|CallParentFunction))

(event Collision|EventActorBeginOverlap
  (params (OtherActor :type Actor%20Object%20Reference)))

(event EventTick
  (params (DeltaSeconds :type Float%20%28single-precision%29))
  (|CallParentFunction DeltaSeconds)
  ;[1 1 1] Added 11/03/2020 - spawn pools underfeet
  (Utilities|FlowControl|Delay 0.5)
  (CallFunction|SpawnPool))

(fn ConstructionScript
  (|CallParentFunction))