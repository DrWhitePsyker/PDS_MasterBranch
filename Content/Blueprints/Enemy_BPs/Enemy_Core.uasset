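; Enemy actor that spots the player and moves to a preferred standoff distance.
; On BeginPlay it registers with Enemy_Manager and caches BP_Character, or destroys itself without a valid manager.
; Update_PlayerSight enters combat on an unobstructed, close-range visibility trace that ignores other enemies.
; In combat, Tick computes the standoff point once (Haspath never resets) and calls AIMoveTo only while the ideal point stays within ShuffleSpace of it.
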(event Custom|Update_PlayerSight
  (bind _returnvalue (Transformation|GetActorLocation))
  (bind _player_pointer (Variables|Default|GetPlayer%20Pointer))
  (bind _outactors (Actor|GetAllActorsOfClass "Enemy_Core_C"))
  (bind _outhit (Collision|LineTraceByChannel (Math|Vector|MakeVector (.x _returnvalue) (.y _returnvalue) (+ (.z _returnvalue) 5e+01)) (Transformation|GetWorldLocation (Variables|/Game/Blueprints/Player_BPs/BP_Character.BP_Character_C|GetCharacter (Variables|Default|GetPlayer%20Pointer))) "TraceTypeQuery1" false _outactors "ForDuration" true "(R=1.000000,G=0.000000,B=0.000000,A=1.000000)" "(R=0.000000,G=1.000000,B=0.000000,A=1.000000)" 0.1))
  (if (and (== (.hitactor _outhit) _player_pointer) (< (Transformation|GetDistanceTo self _player_pointer) 5e+02))
    (Variables|Default|SetInCombat? true)
    (Development|PrintString "PLAYER SPOTTED. ATTACKING!")))

(event EventTick
  (params (DeltaSeconds :type Float%20%28single-precision%29))
  (bind _self self)
  (bind _player_pointer (Variables|Default|GetPlayer%20Pointer))
  (bind _prefered_distance (Variables|Default|GetPrefered%20distance))
  (bind _player_pointer_2 (Variables|Default|GetPlayer%20Pointer))
  (bind _returnvalue (Transformation|GetActorLocation _player_pointer))
  (bind _returnvalue_2 (Transformation|GetActorLocation _self))
  (bind _returnvalue_3 (Transformation|GetActorLocation _player_pointer_2))
  (bind _returnvalue_4 (Math|Vector|GetUnitDirection(Vector) _returnvalue_2 _returnvalue_3))
  (bind _returnvalue_5 (* (.y _returnvalue_4) _prefered_distance))
  (bind _returnvalue_6 (* (.x _returnvalue_4) _prefered_distance))
  (bind _returnvalue_7 (* _returnvalue_5 -1.0))
  (bind _returnvalue_8 (* _returnvalue_6 -1.0))
  (bind _returnvalue_9 (Math|Vector|MakeVector _returnvalue_8 _returnvalue_7 0.0))
  (bind _returnvalue_10 (+ _returnvalue _returnvalue_9))
  (if (Variables|Default|GetInCombat?)
    (if (Variables|Default|Gethaspath?)
      _
      (else
        (bind _output_get (Variables|Default|SetPrecalc%20point _returnvalue_10))
        (Variables|Default|Sethaspath? true)
        (Rendering|Debug|DrawDebugPoint _output_get 5.0 "(R=0.000000,G=0.000000,B=0.000000,A=1.000000)" 0.1)))
    (if (> (Math|Float|Absolute(Float) (Math|Vector|Distance(Vector) (Variables|Default|GetPrecalc%20point) _returnvalue_10)) (Variables|Default|GetShuffle%20space))
      (Variables|Default|Sethaspath? true)
      (else
        (AI|AIMoveTo self (Variables|Default|GetPrecalc%20point) 0 5.0 false)))))

(event EventBeginPlay
  (bind _outactors (Actor|GetAllActorsOfClass "/Game/Blueprints/Enemy_BPs/Enemy_Manager.Enemy_Manager_C"))
  (bind _output_get (Variables|Default|SetEnemy%20Manager%20Pointer (Utilities|Array|Get(acopy) _outactors)))
  (if (Utilities|IsValid _output_get)
    (bind _asenemy_manager (Utilities|Casting|CastToEnemy_Manager (Variables|Default|GetEnemy%20Manager%20Pointer)))
    (Variables|/Game/Blueprints/Enemy_BPs/Enemy_Manager.Enemy_Manager_C|SetEnemyNeedingSorting _asenemy_manager self)
    (Default|FeedtoUpdateArray _asenemy_manager)
    (bind _outactors_2 (Actor|GetAllActorsOfClass "/Game/Blueprints/Player_BPs/BP_Character.BP_Character_C"))
    (Variables|Default|SetPlayer%20Pointer (Utilities|Array|Get(acopy) _outactors_2))
    (else
      (Development|PrintString (Utilities|String|Append (Utilities|String|Append "ERROR IN: " (Utilities|GetDisplayName self)) "  # enemy manager pointer invalid. Is there an enemy manager active?"))
      (Actor|DestroyActor))))

(fn ConstructionScript)