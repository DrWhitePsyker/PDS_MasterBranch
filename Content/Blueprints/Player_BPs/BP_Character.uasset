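; BP_Character is the player character, with world-axis movement, controller yaw turning, hold-to-sprint and automatic shooting.
; BeginPlay spawns a steep overhead BP_Camera targeting the character; Tick accumulates time while Shoot is held to fire BP_RegularBullet at intervals.
; A ChangetoMachineGun event spawns a machine-gun bullet, but Tick forces RegularMode on every frame.
; TakeDamage decrements and prints Health, though its pool-overlap caller is disconnected.
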(event Custom|Change%20to%20Machine%20Gun
  (if (Variables|Default|GetRegularMode)
    (Variables|Default|SetMachineGunMode false)
    (Game|SpawnActorfromClass "/Game/Blueprints/Player_BPs/ShotModes/BP_MachineGunBullet.BP_MachineGunBullet_C" (Transformation|GetActorTransform) "Undefined" 0 self)
    (else
      (Variables|Default|SetRegularMode true)
      (Development|PrintString "Still regular mode"))))

(event EventBeginPlay
  (bind _returnvalue (Transformation|GetActorLocation))
  ;[1 1 1] Character & Camera Spawn
  (bind _returnvalue_2 (Game|SpawnActorfromClass "/Game/Blueprints/Player_BPs/BP_Camera.BP_Camera_C" (Math|Transform|MakeTransform (Math|Vector|MakeVector (- (.x _returnvalue) 2e+02) (.y _returnvalue) (+ (.z _returnvalue) 7e+02)) "-80.000000, 0,0.000000" "1,1,1") "Undefined" 0 0))
  (Variables|/Game/Blueprints/Player_BPs/BP_Camera.BP_Camera_C|Setplayertarget _returnvalue_2 self)
  (Input|EnableInput (Game|GetPlayerController 0))
  (Variables|/Script/Engine.CharacterMovementComponent|SetMaxWalkSpeed (Variables|Character|GetCharacterMovement) (Variables|Default|GetWalk%20Speed))
  (Variables|Default|SetHealth (Variables|Default|GetHealth)))

(event EventTick
  (params (DeltaSeconds :type Float%20%28single-precision%29))
  (Variables|Default|SetRegularMode true)
  (if (Variables|Default|GetShotheld)
    (bind _output_get (Variables|Default|SetShottimeDelta (+ (Variables|Default|GetShottimeDelta) DeltaSeconds)))
    (if (>= _output_get (Variables|Default|GetShotTime))
      (Variables|Default|SetShottimeDelta 0.0)
      (Game|SpawnActorfromClass "/Game/Blueprints/Player_BPs/ShotModes/BP_RegularBullet.BP_RegularBullet_C" (Transformation|GetActorTransform) "Undefined" 0 self)
      (Development|PrintString "Regular Mode"))))

(event Input|ActionEvents|InputActionShoot
  (params (Key :type Key%20Structure :default "None"))
  (:Pressed
    (Variables|Default|SetShotheld true))
  (:Released
    (Variables|Default|SetShotheld false)))

(event Input|ActionEvents|InputActionRun
  (params (Key :type Key%20Structure :default "None"))
  (bind _charactermovement (Variables|Character|GetCharacterMovement))
  (:Pressed
    (Variables|/Script/Engine.CharacterMovementComponent|SetMaxWalkSpeed _charactermovement (Variables|Default|GetSprint%20Speed)))
  (:Released
    (Variables|/Script/Engine.CharacterMovementComponent|SetMaxWalkSpeed _charactermovement (Variables|Default|GetWalk%20Speed))))

(event Input|AxisEvents|InputAxisTurn
  (params (AxisValue :type Float%20%28single-precision%29))
  ;[1 1 1] Movement Funtionality
  (Pawn|Input|AddControllerYawInput AxisValue))

(event Input|AxisEvents|InputAxisMoveright
  (params (AxisValue :type Float%20%28single-precision%29))
  ;[1 1 1] Movement Funtionality
  (Pawn|Input|AddMovementInput "0.000000,1.000000, 0" AxisValue true))

(event Input|AxisEvents|InputAxisMoveForward
  (params (AxisValue :type Float%20%28single-precision%29))
  ;[1 1 1] Movement Funtionality
  (Pawn|Input|AddMovementInput "1.000000, 0, 0" AxisValue true))

(fn ConstructionScript)

(fn Sprint)

(fn TakeDamage
  ;[1 1 1] Decrease health by 1 for each instance of damage taken
  (Math|Integer|DecrementInt (Variables|Default|GetHealth)
    (:%20%20
      (Development|PrintString (Utilities|String|ToString(Integer) (Variables|Default|GetHealth))))))