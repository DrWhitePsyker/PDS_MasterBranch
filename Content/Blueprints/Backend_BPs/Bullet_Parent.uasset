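; Base projectile actor that flies forward and notifies whatever it hits before destroying itself.
; Each tick it makes a swept move along its forward vector, scaling X and Y by Velocity and delta time but leaving Z unscaled.
; On overlap it ignores its instigator and Bullet_Parent actors, sends the NewFunction0 interface message to any other actor, then destroys itself.
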(event EventBeginPlay
  (Variables|Default|SetOrigin (Game|GetInstigator)))

(event EventTick
  (params (DeltaSeconds :type Float%20%28single-precision%29))
  (bind _returnvalue (Transformation|GetActorForwardVector))
  (bind _velocity (Variables|Default|GetVelocity))
  (bind _returnvalue_2 (* _velocity DeltaSeconds))
  (Class|Actor|AddActorWorldTransform (Math|Transform|MakeTransform (Math|Vector|MakeVector (* (.x _returnvalue) _returnvalue_2) (* (.y _returnvalue) _returnvalue_2) (.z _returnvalue)) "0, 0, 0" "1,1,1") true false))

(event Collision|EventActorBeginOverlap
  (params (OtherActor :type Actor%20Object%20Reference))
  (Variables|Default|SetHitActor OtherActor)
  (if (not (or (== (Variables|Default|GetHitActor) (Variables|Default|GetOrigin)) (== (Utilities|GetClass (Variables|Default|GetHitActor)) "Bullet_Parent_C")))
    (bind _asactor (Utilities|Casting|CastToActor (Variables|Default|GetHitActor))
      (:then
        (Class|BulletImpactHandler|NewFunction0(Message) _asactor))
      (:CastFailed
        _))
    (Actor|DestroyActor)))

(fn ConstructionScript)