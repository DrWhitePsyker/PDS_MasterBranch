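; World generator actor that builds a level at BeginPlay as a straight line of rooms, with the room count derived from LevelNumber.
; RoomSpawn calls itself recursively, reading each room's class and length from the RoomDatabase data table and spawning it along negative X.
; It advances by half a length before and after each spawn to butt rooms end to end.
; The row is currently fixed; the random roll is unconnected.
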(event Custom|RoomSpawn
  (if (> (Variables|Default|GetRooms%20remaining) 0)
    (bind _output_get (Variables|Default|SetLevel%20ID%20rolled 1))
    (bind _returnvalue (Utilities|GetDataTableRow "/Game/Blueprints/Enviro_BP/Rooms/RoomDatabase.RoomDatabase" (Utilities|String|StringToName (Utilities|String|ToString(Integer) _output_get)))
      (:then
        (bind _output_get_2 (Variables|Default|SetSizeToShift (/ (.RoomLength (Utilities|Struct|BreakRoomStruct _returnvalue)) 2)))
        (bind _output_get_3 (Variables|Default|SetX%20point (+ (Variables|Default|GetX%20point) _output_get_2)))
        (bind _output_get_4 (Variables|Default|Setspawnpostion (Math|Transform|MakeTransform (Math|Vector|MakeVector (Math|Conversions|ToFloat(Integer) (* _output_get_3 -1)) 0.0 0.0) "0, 0, 0" "1,1,1")))
        (Game|SpawnActorfromClass (.RoomID (Utilities|Struct|BreakRoomStruct _returnvalue)) _output_get_4 "Undefined" 0 0)
        (Variables|Default|SetX%20point (+ (Variables|Default|GetX%20point) (Variables|Default|GetSizeToShift)))
        (Math|Integer|DecrementInt (Variables|Default|GetRooms%20remaining)
          (:%20%20
            (CallFunction|RoomSpawn))))
      (:RowNotFound
        (Development|PrintString "what the fuck")))))

(event EventBeginPlay
  (Variables|Default|SetRooms%20remaining (+ (Variables|Default|GetLevelNumber) 2))
  (Development|PrintString "SPAWN START ROOM")
  (CallFunction|RoomSpawn))

(event Collision|EventActorBeginOverlap
  (params (OtherActor :type Actor%20Object%20Reference)))

(event EventTick
  (params (DeltaSeconds :type Float%20%28single-precision%29)))

(fn ConstructionScript)